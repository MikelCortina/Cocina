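; BP_ProcessingStation is a station that shows its current state on a colored text label.
; State requests broadcast EV_ApplyStationState to all clients as a Photon Fusion custom RPC when in a room, otherwise apply locally.
; Applying a state stores it and refreshes the label: green "Libre" (free), yellow "Procesando" (processing), or red for other states, which also read "Procesando".
; No processing logic lives here.
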(event Custom|SetStationState
  (params (NewState :type Integer))
  (CallFunction|EVApplyStationStateCall NewState))

(event Custom|EV_ApplyStationState
  (params (NewState :type Integer))
  (Variables|Default|SetStationState NewState)
  (CallFunction|UpdateStationVisuals))

(event Custom|RequestApplyStationState
  (params (NewSate :type Integer))
  (CallFunction|EVApplyStationStateCall NewSate))

(event EventBeginPlay)

(event Collision|EventActorBeginOverlap
  (params (OtherActor :type Actor%20Object%20Reference)))

(event EventTick
  (params (DeltaSeconds :type Float%20%28single-precision%29)))

(fn ConstructionScript)

(fn UpdateStationVisuals
  (bind _returnvalue (Utilities|Text|MakeLiteralText "Procesando"))
  (bind _stationstatetext (Variables|Default|GetStationStateText))
  (bind _stationstatetext_2 (Variables|Default|GetStationStateText))
  (if (== (Variables|Default|GetStationState) 0)
    (Rendering|Components|TextRender|SetText (Variables|Default|GetStationStateText) (Utilities|Text|MakeLiteralText "Libre"))
    (Rendering|Components|TextRender|SetTextRenderColor (Variables|Default|GetStationStateText) (Math|Conversions|ToColor(LinearColor) (Utilities|Struct|MakeLinearColor 0.0 1.0 0.0 1.0)))
    (elif (== (Variables|Default|GetStationState) 1)
      (Rendering|Components|TextRender|SetText _stationstatetext _returnvalue)
      (Rendering|Components|TextRender|SetTextRenderColor _stationstatetext (Math|Conversions|ToColor(LinearColor) (Utilities|Struct|MakeLinearColor 1.0 1.0 0.0 1.0)))
      (else
        (Rendering|Components|TextRender|SetText _stationstatetext_2 _returnvalue)
        (Rendering|Components|TextRender|SetTextRenderColor _stationstatetext_2 (Math|Conversions|ToColor(LinearColor) (Utilities|Struct|MakeLinearColor 1.0 0.0 0.0 1.0)))))))

(fn EVApplyStationStateCall
  (params (NewState :type Integer))
  (bind _self self)
  (bind _parambuffer (LocalVariables|GetParamBuffer))
  (if (Class|FusionOnlineSubsystem|IsinRoom (Subsystems|GetFusionOnlineSubsystem))
    (bind _returnvalue (Class|FusionHelpers|GetFunctionDescriptor _self "EV_ApplyStationState"))
    (if (Utilities|IsValid _returnvalue)
      (Class|FusionHelpers|AddParamtoBuffer NewState _self _returnvalue 0 _parambuffer)
      (Class|FusionHelpers|InvokeCustomRPC _self "EV_ApplyStationState" 1427379474 "SendToAllClients" _parambuffer))
    (else
      (CallFunction|EVApplyStationState NewState))))
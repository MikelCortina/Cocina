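; BP_MenuSessionFlow is an actor that connects the game to Photon and enters a multiplayer room.
; CreateRoomFlow and JoinRoomFlow share identical logic: connect, then join or create a four-player Lvl_ThirdPerson room using the PJR_GameInstance room name.
; JoinOrCreateRoom is wired to both the immediate and success outputs of ConnectToPhoton, so it can fire before connection completes.
; Progress and failures appear only as printed debug strings.
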(event Custom|JoinRoomFlow
  (Development|PrintString "BP_MenuSessionFlow: Unirse a sala")
  (bind _aspjr_game_instance (Utilities|Casting|CastToPJR_GameInstance (Game|GetGameInstance)))
  (|ConnecttoPhoton
    (:then
      (bind _code (|JoinorCreateRoom (Utilities|Struct|MakeFusionRoomOptions (Class|PJRGameInstance|GetRoomName _aspjr_game_instance) 0 5 4 true true "/Game/ThirdPerson/Lvl_ThirdPerson.Lvl_ThirdPerson") :!label _label)
        (:OnFailure
          (Development|PrintString (Utilities|String|EnumtoString _code) :!label _label_2))
        (:OnSuccess
          (Development|PrintString "Conectado a sala correctamente"))))
    (:OnFailure
      (goto _label_2))
    (:OnSuccess
      (Development|PrintString "Conectado a Photon")
      (goto _label))))

(event Custom|CreateRoomFlow
  (Development|PrintString "BP_MenuSessionFlow: Crear sala")
  (bind _aspjr_game_instance (Utilities|Casting|CastToPJR_GameInstance (Game|GetGameInstance)))
  (|ConnecttoPhoton
    (:then
      (bind _code (|JoinorCreateRoom (Utilities|Struct|MakeFusionRoomOptions (Class|PJRGameInstance|GetRoomName _aspjr_game_instance) 0 5 4 true true "/Game/ThirdPerson/Lvl_ThirdPerson.Lvl_ThirdPerson") :!label _label)
        (:OnFailure
          (Development|PrintString (Utilities|String|EnumtoString _code) :!label _label_2))
        (:OnSuccess
          (Development|PrintString "Conectado a sala correctamente"))))
    (:OnFailure
      (goto _label_2))
    (:OnSuccess
      (Development|PrintString "Conectado a Photon")
      (goto _label))))

(event EventBeginPlay)

(event Collision|EventActorBeginOverlap
  (params (OtherActor :type Actor%20Object%20Reference)))

(event EventTick
  (params (DeltaSeconds :type Float%20%28single-precision%29)))

(fn ConstructionScript)
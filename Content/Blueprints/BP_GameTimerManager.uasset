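; Match manager actor for a networked game that runs the countdown, tracks the score and shows both on text components.
; The room creator ticks the timer each second; time and score changes broadcast through Fusion custom RPCs, or apply locally outside a room.
; Timeout or recipe completion ends the match and opens WBP_EndMatch, with only the recipe path passing it the score.
; Non-creators route recipe-end requests through the master client, which rebroadcasts them.
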(event Custom|EV_TimerTick
  (CallFunction|TickTimer))

(event Custom|RequestTimerTick
  (if (not (Variables|Default|GetMatchEnded))
    (CallFunction|EVApplyTimerValueCall (- (Variables|Default|GetTimeRemaining) 1))))

(event Custom|EV_ApplyTimerValue
  (params (NewTime :type Integer))
  (bind _returnvalue (Game|GetPlayerController 0))
  (Variables|Default|SetTimeRemaining NewTime)
  (CallFunction|UpdateTimerVisuals)
  (if (<= NewTime 0)
    (Variables|Default|SetMatchEnded true)
    (Development|PrintString "Fin de partida")
    (Development|PrintString (Utilities|String|Append "Puntuación final: " (Utilities|String|ToString(Integer) (Variables|Default|GetScore))))
    (bind _returnvalue_2 (UserInterface|CreateWidget "/Game/UI/WBP_EndMatch.WBP_EndMatch_C" (Game|GetPlayerController 0)))
    (UserInterface|Viewport|AddtoViewport _returnvalue_2 0)
    (Variables|/Script/Engine.PlayerController|SetbShowMouseCursor _returnvalue true)
    (Input|SetInputModeUIOnly _returnvalue _returnvalue_2 "DoNotLock" false)))

(event Custom|EV_ApplyScoreValue
  (params (NewScore :type Integer))
  (Variables|Default|SetScore NewScore)
  (CallFunction|UpdateScoreVisuals))

(event Custom|RequestAddScore
  (params (PointsToAdd :type Integer))
  (CallFunction|EVApplyScoreValueCall (+ (Variables|Default|GetScore) PointsToAdd)))

(event Custom|EndMatchByRecipe
  (Variables|Default|SetMatchEnded true)
  (Development|PrintString "Partida finalizada por receta"))

(event Custom|EV_EndMatchByRecipe
  (Development|PrintString "RPC FINAL EJECUTADO")
  (Variables|Default|SetMatchEnded true)
  (Development|PrintString "Partida finalizada por receta")
  (bind _returnvalue (UserInterface|CreateWidget "/Game/UI/WBP_EndMatch.WBP_EndMatch_C"))
  (Default|SetFinalScore _returnvalue (Variables|Default|GetScore))
  (UserInterface|Viewport|AddtoViewport _returnvalue 0))

(event Custom|RequestEndMatchByRecipe
  (bind _asbp_pjr_game_instance (Utilities|Casting|CastToBP_PJR_GameInstance (Game|GetGameInstance)))
  (if (Variables|/Game/Blueprints/BP_PJR_GameInstance.BP_PJR_GameInstance_C|GetIsRoomCreator _asbp_pjr_game_instance)
    (CallFunction|EVEndMatchbyRecipeCall)
    (else
      (CallFunction|EVRequestEndMatchbyRecipeCall))))

(event Custom|EV_RequestEndMatchByRecipe
  (Development|PrintString "\"HOST RECIBE PETICION DE FINAL\"")
  (CallFunction|EVEndMatchbyRecipeCall))

(event EventBeginPlay
  (CallFunction|UpdateTimerVisuals)
  (bind _asbp_pjr_game_instance (Utilities|Casting|CastToBP_PJR_GameInstance (Game|GetGameInstance)))
  (if (Variables|/Game/Blueprints/BP_PJR_GameInstance.BP_PJR_GameInstance_C|GetIsRoomCreator _asbp_pjr_game_instance)
    (Utilities|Time|SetTimerbyFunctionName 0 "RequestTimerTick" 1.0 true)))

(event Collision|EventActorBeginOverlap
  (params (OtherActor :type Actor%20Object%20Reference)))

(event EventTick
  (params (DeltaSeconds :type Float%20%28single-precision%29)))

(fn ConstructionScript)

(fn OnRepTimeRemaining)

(fn OnRepMatchEnded)

(fn UpdateTimerVisuals
  (Rendering|Components|TextRender|SetText (Variables|Default|GetTimerText) (|GenerictoText (Utilities|String|Append "Tiempo: " (Utilities|String|ToString(Integer) (Variables|Default|GetTimeRemaining))))))

(fn TickTimer
  (if (not (Variables|Default|GetMatchEnded))
    (Variables|Default|SetTimeRemaining (- (Variables|Default|GetTimeRemaining) 1))
    (CallFunction|UpdateTimerVisuals)
    (if (<= (Variables|Default|GetTimeRemaining) 0)
      (Variables|Default|SetMatchEnded true)
      (Development|PrintString "\"Fin de partida\""))))

(fn EVApplyTimerValueCall
  (params (NewTime :type Integer))
  (bind _self self)
  (bind _parambuffer (LocalVariables|GetParamBuffer))
  (if (Class|FusionOnlineSubsystem|IsinRoom (Subsystems|GetFusionOnlineSubsystem))
    (bind _returnvalue (Class|FusionHelpers|GetFunctionDescriptor _self "EV_ApplyTimerValue"))
    (if (Utilities|IsValid _returnvalue)
      (Class|FusionHelpers|AddParamtoBuffer NewTime _self _returnvalue 0 _parambuffer)
      (Class|FusionHelpers|InvokeCustomRPC _self "EV_ApplyTimerValue" 338504446 "SendToAllClients" _parambuffer))
    (else
      (CallFunction|EVApplyTimerValue NewTime))))

(fn OnRepScore)

(fn UpdateScoreVisuals
  (Rendering|Components|TextRender|SetText (Variables|Default|GetScoreText) (|GenerictoText (Utilities|String|Append " Score: " (Utilities|String|ToString(Integer) (Variables|Default|GetScore))))))

(fn EVApplyScoreValueCall
  (params (NewScore :type Integer))
  (bind _self self)
  (bind _parambuffer (LocalVariables|GetParamBuffer))
  (if (Class|FusionOnlineSubsystem|IsinRoom (Subsystems|GetFusionOnlineSubsystem))
    (bind _returnvalue (Class|FusionHelpers|GetFunctionDescriptor _self "EV_ApplyScoreValue"))
    (if (Utilities|IsValid _returnvalue)
      (Class|FusionHelpers|AddParamtoBuffer NewScore _self _returnvalue 0 _parambuffer)
      (Class|FusionHelpers|InvokeCustomRPC _self "EV_ApplyScoreValue" 1304340999 "SendToAllClients" _parambuffer))
    (else
      (CallFunction|EVApplyScoreValue NewScore))))

(fn EVEndMatchbyRecipeCall
  (bind _self self)
  (if (Class|FusionOnlineSubsystem|IsinRoom (Subsystems|GetFusionOnlineSubsystem))
    (bind _returnvalue (Class|FusionHelpers|GetFunctionDescriptor _self "EV_EndMatchByRecipe"))
    (if (Utilities|IsValid _returnvalue)
      (Class|FusionHelpers|InvokeCustomRPC _self "EV_EndMatchByRecipe" 1970972876 "SendToAllClients" (LocalVariables|GetParamBuffer)))
    (else
      (CallFunction|EVEndMatchbyRecipe))))

(fn EVRequestEndMatchbyRecipeCall
  (bind _self self)
  (if (Class|FusionOnlineSubsystem|IsinRoom (Subsystems|GetFusionOnlineSubsystem))
    (bind _returnvalue (Class|FusionHelpers|GetFunctionDescriptor _self "EV_RequestEndMatchByRecipe"))
    (if (Utilities|IsValid _returnvalue)
      (Class|FusionHelpers|InvokeCustomRPC _self "EV_RequestEndMatchByRecipe" 1726322686 "SendToMasterClient" (LocalVariables|GetParamBuffer)))
    (else
      (CallFunction|EVRequestEndMatchbyRecipe))))
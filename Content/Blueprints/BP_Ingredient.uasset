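; Networked ingredient actor that can be picked up, which hides it and disables its collision.
; A pickup request goes out as a Photon Fusion custom RPC to all clients when in a room, otherwise it runs locally.
; The pickup sets IsPickedUp, whose OnRep handler runs the same visibility and collision update.
; BeginPlay also creates and stores a dynamic instance of the ingredient material.
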(event Custom|EV_PickUpIngredient
  (CallFunction|PickUp))

(event Custom|RequestPickUpIngredient
  (CallFunction|EVPickUpIngredientCall) ; RPC_PickUpIngredient
)

(event EventBeginPlay
  (bind _returnvalue (Rendering|Material|CreateDynamicMaterialInstance "/Game/Blueprints/Mt_Ingredient.Mt_Ingredient" "None" "None" :!class /Script/Engine.KismetMaterialLibrary))
  (Variables|Default|SetDynamicMaterial _returnvalue))

(event Collision|EventActorBeginOverlap
  (params (OtherActor :type Actor%20Object%20Reference)))

(event EventTick
  (params (DeltaSeconds :type Float%20%28single-precision%29)))

(fn ConstructionScript)

(fn OnRepIsPickedUp
  (CallFunction|UpdateIngredientVisuals))

(fn PickUp
  (Variables|Default|SetIsPickedUp true)
  (CallFunction|UpdateIngredientVisuals))

(fn UpdateIngredientVisuals
  (if (Variables|Default|GetIsPickedUp)
    (Rendering|SetActorHiddenInGame true)
    (Collision|SetActorEnableCollision false)
    (else
      (Rendering|SetActorHiddenInGame false)
      (Collision|SetActorEnableCollision true))))

(fn EVPickUpIngredientCall
  (bind _self self)
  (if (Class|FusionOnlineSubsystem|IsinRoom (Subsystems|GetFusionOnlineSubsystem))
    (bind _returnvalue (Class|FusionHelpers|GetFunctionDescriptor _self "EV_PickUpIngredient"))
    (if (Utilities|IsValid _returnvalue)
      (Class|FusionHelpers|InvokeCustomRPC _self "EV_PickUpIngredient" 1070139814 "SendToAllClients" (LocalVariables|GetParamBuffer)))
    (else
      (CallFunction|EVPickUpIngredient))))
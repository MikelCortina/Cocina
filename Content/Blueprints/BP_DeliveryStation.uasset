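; Delivery station that counts delivered ingredients and shows the total on its ScoreText label.
; DeliverIngredient increments DeliveredCount and calls UpdateStationVisuals, which writes the count after the "Entregas:" prefix.
; DeliveredCount uses a RepNotify that runs the same refresh when the value replicates.
; The event graph is empty, and DeliverIngredient has no caller or authority check in this Blueprint.
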(event EventBeginPlay)

(event Collision|EventActorBeginOverlap
  (params (OtherActor :type Actor%20Object%20Reference)))

(event EventTick
  (params (DeltaSeconds :type Float%20%28single-precision%29)))

(fn ConstructionScript)

(fn OnRepDeliveredCount
  (CallFunction|UpdateStationVisuals))

(fn UpdateStationVisuals
  (Rendering|Components|TextRender|SetText (Variables|Default|GetScoreText) (|GenerictoText (Utilities|String|Append "Entregas: " (Utilities|String|ToString(Integer) (Variables|Default|GetDeliveredCount))))))

(fn DeliverIngredient
  (Variables|Default|SetDeliveredCount (+ (Variables|Default|GetDeliveredCount) 1))
  (CallFunction|UpdateStationVisuals))